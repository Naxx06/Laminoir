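; BP_BaseKey is a configurable key pickup actor that adds its key ID to the player's door keys.
; The construction script applies the configured mesh and scale, while interface-style functions report interactability and the prompt name.
; On Interact, it shows a colored HUD notification, appends KeyID to the DoorKeys of the player reference cached at BeginPlay, plays an attenuated pickup sound, and destroys itself.
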(event EventInteract
  (params (Player :type BP%20Player%20Perso%20Object%20Reference))
  ;[0.05098 0.05098 0.05098] Key function
  (Default|AddNotification (Variables|/Game/FPMovement/Player/Blueprints/BP_PlayerPerso.BP_PlayerPerso_C|GetWP_PlayerHUD Player) (Variables|KeySettings|GetPickup%20Notification) (Utilities|Text|ToText(Name) (Variables|KeySettings|GetKey%20Name)) (Variables|KeySettings|GetItem%20Color%20Notification))
  (Utilities|Array|Add (Variables|/Game/FPMovement/Player/Blueprints/BP_PlayerPerso.BP_PlayerPerso_C|GetDoorKeys (Variables|Reference|GetPlayer%20Reference)) (Variables|KeySettings|GetKeyID))
  (CallFunction|PlayPickupSFX)
  (Actor|DestroyActor))

(event EventBeginPlay
  ;[0.05098 0.05098 0.05098] Cast to Player
  (bind _asbp_player (Utilities|Casting|CastToBP_PlayerPerso (Game|GetPlayerCharacter 0)))
  (Variables|Reference|SetPlayer%20Reference _asbp_player))

(fn ConstructionScript
  (Components|StaticMesh|SetStaticMesh (Variables|Default|GetItem) (Variables|KeySettings|GetKey%20Mesh))
  (Transformation|SetWorldScale3D (Variables|Default|GetItem) (Math|Conversions|ToVector(Float) (Variables|KeySettings|GetKey%20Scale))))

(fn CanInteract?
  (return (Variables|PRIVAT|GetCanInteract?)))

(event Custom|Play%20Pickup%20SFX
  (Audio|PlaySoundatLocation (Variables|ItemSFX|GetPickup%20SFX) (Transformation|GetWorldLocation (Variables|Default|GetItem)) "0, 0, 0" (Variables|ItemSFX|GetPickup%20Volume) 1.0 0.0 "/Game/FPMovement/Assets/Audio/Abilitys/Pickup/Effects/ItemAttenuation.ItemAttenuation" 0 0 0))

(fn InteractPrompt
  (return (Variables|KeySettings|GetShow%20Key%20Prompt?) (Variables|KeySettings|GetKey%20Name)))