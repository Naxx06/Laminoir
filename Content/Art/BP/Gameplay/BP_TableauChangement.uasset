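; BP_TableauChangement is a painting actor that changes its picture whenever it leaves view after being seen.
; A looping timer started on BeginPlay polls whether the canvas mesh was recently rendered.
; When a seen canvas stops rendering, it applies the next material from a painting array, wrapping around, then waits to be seen again.
; Visibility relies on WasRecentlyRendered rather than traces or camera-angle checks.
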(event Custom|CheckPaintingVisibility
  (if (Class|PrimitiveComponent|WasRecentlyRendered (Variables|Default|GetCanvaMesh) 0.2)
    (Variables|Default|SetWasLookingAtPainting true)
    (elif (Variables|Default|GetWasLookingAtPainting)
      (Variables|Default|SetCurrentPaintingIndex (Math|Integer|%(Integer) (+ (Variables|Default|GetCurrentPaintingIndex) 1) (Utilities|Array|Length (Variables|Default|GetPaintingMaterials))))
      (Rendering|Material|SetMaterial (Variables|Default|GetCanvaMesh) 0 (Utilities|Array|Get(acopy) (Variables|Default|GetPaintingMaterials) (Variables|Default|GetCurrentPaintingIndex)))
      (Variables|Default|SetWasLookingAtPainting false))))

(event EventBeginPlay
  (Utilities|Time|SetTimerbyEvent (delegate Custom|CheckPaintingVisibility) 0.15 true))

(fn ConstructionScript)