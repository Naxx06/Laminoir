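; Level sequence controller that stages the scripted mirror-door reveal and the corridor's secret-painting progression.
; BeginPlay hides the reveal props, then player triggers advance a gameplay state to open the maintenance door, show the painting and slam the mirror door.
; The one-shot reveal times a fake-door animation, sounds and camera fade to mask the wall swap.
; It binds to the streamed mirror level's shown event to find spotlight and fake door by tag.
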(event OnComponentBeginOverlap(TriggerBox)
  (params (OverlappedComponent :type Primitive%20Component%20Object%20Reference) (OtherActor :type Actor%20Object%20Reference) (OtherComp :type Primitive%20Component%20Object%20Reference) (OtherBodyIndex :type Integer) (bFromSweep :type Boolean) (SweepResult :type Hit%20Result%20Structure%20%28by%20ref%29))
  (bind _returnvalue (Game|GetPlayerController 0))
  (bind _playercameramanager (Variables|/Script/Engine.PlayerController|GetPlayerCameraManager _returnvalue))
  (Utilities|Casting|CastToBP_PlayerPerso OtherActor)
  (if (not (Variables|Default|GetSequenceAlreadyPlayed))
    (Variables|Default|SetSequenceAlreadyPlayed true)
    (Default|StartfakeDoorAnimation (Variables|Default|GetFakedoor))
    (Audio|PlaySoundatLocation "/Game/Art/Sounds/FX_Aveugle_WoodenDoorCreek.FX_Aveugle_WoodenDoorCreek" (Transformation|GetActorLocation (Variables|Default|GetDoorActor)) "0, 0, 0" 1.0 1.0 0.0 0 0 0 0)
    (Utilities|FlowControl|Delay 8.02)
    (Rendering|SetActorHiddenInGame (Variables|Default|GetSpotLightActor) true)
    (Audio|PlaySoundatLocation "/Game/Art/BP/Animation_Door_Reflet/FX_Aveuge_1125DoorSlam.FX_Aveuge_1125DoorSlam" (Transformation|GetActorLocation (Variables|Default|GetDoorActor)) "0, 0, 0" 1.0 1.0 0.0 0 0 0 0)
    (CameraFades|StartCameraFade :self _playercameramanager :ToAlpha 1.0 :Duration 0.3 :bHoldWhenFinished true)
    (Utilities|FlowControl|Delay 2.0)
    (Rendering|SetActorHiddenInGame (Variables|Default|GetNormalWallActor) true)
    (CameraFades|StartCameraFade :self _playercameramanager :FromAlpha 1.0 :Duration 0.5)
    (Default|RevealMirrorDoor (Variables|Default|GetDoorActor))))

(event OnActorBeginOverlap(Trigger_world_Mirror)
  (params (OverlappedActor :type Actor%20Object%20Reference) (OtherActor :type Actor%20Object%20Reference))
  (CallFunction|ShowMirrorLevel))

(event OnActorBeginOverlap(Trigger_CloseDoor)
  (params (OverlappedActor :type Actor%20Object%20Reference) (OtherActor :type Actor%20Object%20Reference))
  (Utilities|Casting|CastToBP_PlayerPerso OtherActor)
  (Default|ClaquePorte (Variables|Default|GetDoorActor)))

(event OnActorBeginOverlap(TriggerFirstPassage)
  (params (OverlappedActor :type Actor%20Object%20Reference) (OtherActor :type Actor%20Object%20Reference))
  ;[0.15 0.15 0.15 0.5] Comment
  (Utilities|Casting|CastToBP_PlayerPerso OtherActor)
  (if (Utilities|Enum|Equal(Enum) (Variables|Default|GetCurrentGameplayState) "NewEnumerator0")
    (Variables|Default|SetCurrentGameplayState "NewEnumerator1")
    (Development|PrintString "Premier passage")))

(event OnActorBeginOverlap(Trigger_ReturnCorridor)
  (params (OverlappedActor :type Actor%20Object%20Reference) (OtherActor :type Actor%20Object%20Reference))
  (Utilities|Casting|CastToBP_PlayerPerso OtherActor)
  (if (Utilities|Enum|Equal(Enum) (Variables|Default|GetCurrentGameplayState) "NewEnumerator1")
    (Default|StartDoorAnimationAll (Variables|Default|GetEntretien_Door))
    (Default|ShowPainting (Variables|Default|GetSecretPainting))
    (Variables|Default|SetCurrentGameplayState "NewEnumerator2")
    (Audio|PlaySoundatLocation "/Game/Art/Sounds/Creaky_Door_Open_10.Creaky_Door_Open_10" "-6852.192228,6205.775266,6159.153346" "0, 0, 0" 1.0 1.0 0.0 "/Game/Art/Sounds/Att_Door.Att_Door" 0 0 0)))

(event Custom|Show_Mirror_Level
  (bind _returnvalue (Class|LevelStreamingDynamic|LoadLevelInstance "Slvl_Mirror" "0, 0, 0" "0, 0, 0" "" 0 false))
  (bind _output_get (Variables|Default|SetMirrorLevelstreamin _returnvalue))
  (EventDispatchers|BindEventtoOnLevelShown _output_get (delegate Custom|Initialize_Mirror_References)))

(event Custom|RevealPaintingHole
  (bind _crankref (Variables|Default|GetCrankRef))
  (Rendering|SetActorHiddenInGame (Variables|Default|GetWall_Normal) true)
  (Collision|SetActorEnableCollision (Variables|Default|GetWall_Normal) true)
  (Rendering|SetActorHiddenInGame (Variables|Default|GetWall_trou) false)
  (Rendering|SetActorHiddenInGame _crankref false)
  (Collision|SetActorEnableCollision _crankref true))

(event Custom|Initialize_Mirror_References
  (bind _outactors (Actor|GetAllActorswithTag "Spotlight_Door"))
  (Utilities|IsValid (Utilities|Array|Get(acopy) _outactors)
    (:Is%20Valid
      (bind _asbp_spotlight_reflet (Utilities|Casting|CastToBP_Spotlight_reflet (Utilities|Array|Get(acopy) _outactors)))
      (Variables|Default|SetSpotLightActor _asbp_spotlight_reflet)
      (bind _outactors_2 (Actor|GetAllActorswithTag "Mirror_Door"))
      (Utilities|IsValid (Utilities|Array|Get(acopy) _outactors_2)
        (:Is%20Valid
          (bind _asbp_door_animation (Utilities|Casting|CastToBP_Door_animation (Utilities|Array|Get(acopy) _outactors_2)))
          (Variables|Default|SetFakedoor _asbp_door_animation))))))

(event EventBeginPlay
  (bind _crankref (Variables|Default|GetCrankRef))
  (Default|HideMirrorDoor (Variables|Default|GetDoorActor))
  (Default|HideLamp (Variables|Default|GetWallLampActor))
  (Default|HidePainting (Variables|Default|GetSecretPainting))
  (Rendering|SetActorHiddenInGame (Variables|Default|GetWall_Normal) false)
  (Collision|SetActorEnableCollision (Variables|Default|GetWall_Normal) true)
  (Rendering|SetActorHiddenInGame (Variables|Default|GetWall_trou) true)
  (Rendering|Material|SetMaterial (Variables|/Script/Engine.StaticMeshActor|GetStaticMeshComponent (Variables|Default|GetMirrorMesh)) 0 (Variables|Default|GetMirrorMaterial_Begin))
  (Rendering|SetActorHiddenInGame _crankref true)
  (Collision|SetActorEnableCollision _crankref false))

(event Collision|EventActorBeginOverlap
  (params (OtherActor :type Actor%20Object%20Reference)))

(event EventTick
  (params (DeltaSeconds :type Float%20%28single-precision%29)))

(fn ConstructionScript)