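; Interactable hinged door that can be locked, opened and slammed shut, with a mirror-door mesh shown or hidden by events.
; Interact checks the player's keys against KeyID to unlock with a HUD notification, otherwise plays locked feedback.
; When unlocked, a reversible timeline swings the door, timing sounds by angle and blocking interaction until finished.
; Claque_Porte slams an open door once and relocks it; UnlockDoor unlocks it without a key.
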(event Custom|HideMirrorDoor
  (Rendering|SetVisibility (Variables|Default|GetPorte_etage_11) false true))

(event Custom|Claque_Porte
  (bind _rotatedoor_tl (Variables|Default|GetRotateDoor_TL))
  ;[0.15 0.15 0.15 0.5] Slam_Door
  (if (not (Variables|Default|GetHasSlammed))
    (if (not (Variables|Variables|GetIsClosed))
      (Variables|Default|SetHasSlammed true)
      (bind _alpha (Timeline|TL_Slam PlayFromStart)
        (:Update
          (Transformation|SetRelativeRotation (Variables|Default|GetDoor_real) (Math|Rotator|Lerp(Rotator) (Variables|Default|GetClosedRotation) (Variables|Default|GetOpenRotation) _alpha) false false))
        (:Finished
          (Transformation|SetRelativeRotation (Variables|Default|GetDoor_real) (Variables|Default|GetClosedRotation) false false)
          (Audio|Components|Audio|Stop _rotatedoor_tl)
          (Components|Timeline|SetNewTime _rotatedoor_tl 0.0)
          (Variables|DoorSettings|SetIsLocked true)
          (Variables|Variables|SetIsClosed true)
          (Audio|PlaySoundatLocation "/Game/Art/BP/Animation_Door_Reflet/FX_Aveuge_1125DoorSlam.FX_Aveuge_1125DoorSlam" (Transformation|GetActorLocation) "0, 0, 0" 1.0 1.0 0.0 0 0 0 0))))))

(event Custom|RevealMirrorDoor
  (Rendering|SetVisibility (Variables|Default|GetPorte_etage_11) true true))

(event Custom|UnlockDoor
  (Variables|DoorSettings|SetIsLocked false)
  (Audio|PlaySound2D (Variables|SFXSettings|GetUnlockSound) 1.0 1.0 0.0 0 0))

(event EventInteract
  (params (Player :type BP%20Player%20Perso%20Object%20Reference))
  ;[0.05098 0.05098 0.05098] CheckForKey function
  (if (Variables|DoorSettings|GetIsLocked)
    ;;[0.03065 0.03717 0.05098] Unlock function
    (bind _haskey (CallFunction|CheckforKey (Variables|/Game/FPMovement/Player/Blueprints/BP_PlayerPerso.BP_PlayerPerso_C|GetDoorKeys Player)))
    (if _haskey
      (Variables|DoorSettings|SetIsLocked false)
      (Default|AddNotification (Variables|/Game/FPMovement/Player/Blueprints/BP_PlayerPerso.BP_PlayerPerso_C|GetWP_PlayerHUD Player) (Variables|DoorSettings|Notification|GetUnlock%20Notification) (Variables|DoorSettings|Notification|GetDoor%20Name%20Notification) (Variables|DoorSettings|Notification|GetDoor%20Name%20Color%20Notification))
      (Utilities|FlowControl|DoOnce false
        (:Completed
          (Audio|PlaySoundatLocation (Variables|SFXSettings|GetUnlockSound) (Transformation|GetActorLocation) "0, 0, 0" 0.5 1.0 0.0 "/Game/FPMovement/Assets/Audio/Abilitys/Door/Effects/DoorAttenuation.DoorAttenuation" 0 0 0)))
      (else
        ;[0.05098 0.05098 0.05098] Door Locked function
        (|DoorLocked_2)))
    (else
      ;[0.05098 0.05098 0.05098] Open/Close Door function
      (|Open/CloseDoor_2))))

(event EventBeginPlay)

(fn ConstructionScript)

(fn CheckforKey
  (params (Keys :type Array%20of%20Integers))
  (return (Utilities|Array|ContainsItem Keys (Variables|DoorSettings|GetKeyID))))

(fn CanInteract?
  (return (Variables|PRIVAT|GetCanInteract?)))

(fn InteractPrompt
  (return (Variables|DoorSettings|GetShow%20Door%20Prompt?) (select (Variables|Variables|GetIsClosed) (Variables|DoorSettings|GetDoorCloseText) (Variables|DoorSettings|GetDoorOpenText))))