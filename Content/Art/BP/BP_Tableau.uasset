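; BP_Tableau is an interactable painting that slides aside once to reveal a hole and make a referenced crank usable.
; Interact plays a sound, then on first use notifies the mirror door sequence and runs a timeline that lerps the mesh sideways from its starting relative location.
; The timeline enables the crank's collision and, when finished, disables the painting's own.
; Helper functions show or hide the whole actor with its collision.
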(event EventBeginPlay
  (bind _ukkpdhqbw_tier_2 (Variables|Default|Getukkpdhqbw_tier_2))
  (bind _relativelocation (Variables|/Script/Engine.SceneComponent|GetRelativeLocation _ukkpdhqbw_tier_2))
  (bind _output_get (Variables|Default|SetClosedLocation _relativelocation))
  (bind _output_get_2 (Variables|Default|SetOpenLocation (+ _relativelocation "0.000000,-120.000000,0.000000"))))

(event EventInteract
  (params (Player :type BP%20Player%20Perso%20Object%20Reference))
  (Audio|PlaySound2D "/Game/Art/Sounds/av_coulissedeclic.av_coulissedeclic" 0.7 1.0 0.3 0 0)
  (if (not (Variables|Default|GetPaintingAlreadyOpened))
    (Default|RevealPaintingHole (Variables|Default|GetMiroorDoorSequenceRef))
    (Variables|Default|SetPaintingAlreadyOpened true)
    (bind _alpha (Timeline|TL_SlidePainting PlayFromStart)
      (:Update
        (Transformation|SetRelativeLocation (Variables|Default|Getukkpdhqbw_tier_2) (Math|Vector|Lerp(Vector) (stale EventBeginPlay _output_get) (stale EventBeginPlay _output_get_2) _alpha) false false)
        (Collision|SetActorEnableCollision (Variables|Default|GetCrankRef) true))
      (:Finished
        (Collision|SetActorEnableCollision false)
        (Collision|SetActorEnableCollision (Variables|Default|GetCrankRef) true)))))

(fn ConstructionScript)

(fn HidePainting
  (Rendering|SetActorHiddenInGame true)
  (Collision|SetActorEnableCollision false))

(fn ShowPainting
  (Rendering|SetActorHiddenInGame false)
  (Collision|SetActorEnableCollision true))

(fn CanInteract?
  (return (not (Variables|Default|GetPaintingAlreadyOpened))))

(fn InteractPrompt
  (return true "Déplacer"))