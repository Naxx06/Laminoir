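; Interactable crank receptacle for the gramophone that lets a player carrying the crank insert it once to activate the mirror world.
; Insertion clears the player's crank, reveals the crank mesh and switches the BP_MirrorDoorSequence manager, found at BeginPlay, to its MirrorWorldActivated state.
; A timeline then spins the crank over a clicking sound, ending with a latch click and a shutter sound played at an arrow's location.
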(event EventBeginPlay
  (bind _returnvalue (Actor|GetActorOfClass "/Game/Art/BP/Animation_Door_Reflet/BP_MirrorDoorSequence.BP_MirrorDoorSequence_C"))
  (Variables|Default|SetManagerRef _returnvalue))

(event EventInteract
  (params (Player :type BP%20Player%20Perso%20Object%20Reference))
  ;[0.2989 1 0.1855] Checks
  (bind _asbp_player_perso (Utilities|Casting|CastToBP_PlayerPerso Player))
  (if (not (Variables|Default|GetiscrankInserted))
    (if (Variables|/Game/FPMovement/Player/Blueprints/BP_PlayerPerso.BP_PlayerPerso_C|GetHasCrank Player)
      (Variables|Default|SetiscrankInserted true)
      (Variables|/Game/FPMovement/Player/Blueprints/BP_PlayerPerso.BP_PlayerPerso_C|SetHasCrank _asbp_player_perso false)
      (Rendering|SetVisibility (Variables|Default|GetCrank1) true false)
      ;[0 0 0 0.5] State MirrorWorldActivated
      (Variables|/Game/Art/BP/Animation_Door_Reflet/BP_MirrorDoorSequence.BP_MirrorDoorSequence_C|SetCurrentGameplayState (Variables|Default|GetManagerRef) "NewEnumerator4")
      (Default|ApplyGameplayState (Variables|Default|GetManagerRef))
      ;[1 0.1624 0.1204] Crank noise
      (bind _returnvalue (Audio|SpawnSound2D "/Game/Art/BP/Gramophone/av_cliquetisRoue.av_cliquetisRoue" 1.0 1.0 0.0 0))
      (Variables|Default|SetCrankAudioComponent _returnvalue)
      (bind _rotation (Timeline|TL_RotateCrank Play)
        (:Update
          (Transformation|SetRelativeRotation (Variables|Default|GetCrank1) (Math|Rotator|MakeRotator 0.0 0.0 _rotation) false false))
        (:Finished
          (Audio|PlaySound2D "/Game/Art/Sounds/declic_close1.declic_close1" 1.0 1.0 0.0 0 0)
          (Audio|SpawnSoundatLocation "/Game/Art/Sounds/av_l11_volet1.av_l11_volet1" (Transformation|GetWorldLocation (Variables|Default|GetArrowSoundLocation)) "0, 0, 0" 2.0 1.0 0.0 0 0))))))

(fn ConstructionScript)

(fn CanInteract?
  (return (not (Variables|Default|GetiscrankInserted))))

(fn InteractPrompt
  (return (not (Variables|Default|GetHasbeenActivated)) "Insérer la manivelle"))