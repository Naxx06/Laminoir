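; BP_Crank is an interactable pickup for a crank, filed with the gramophone assets, with a French "pick up the crank" prompt.
; On interact it plays a metal impact sound, sets HasCrank on BP_PlayerPerso, then hides itself and disables its collision and tick.
; CanInteract depends on HasBeenPickedUp, which these graphs never set, so disabled collision is what this file does to block repeat pickups.
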(event EventInteract
  (params (Player :type BP%20Player%20Perso%20Object%20Reference))
  (Audio|PlaySound2D "/Game/Art/BP/Gramophone/BangMetalRailHugeImpactsOnHospitalBed_9mLQY_01.BangMetalRailHugeImpactsOnHospitalBed_9mLQY_01" 0.5 1.0 0.0 0 0)
  (bind _asbp_player_perso (Utilities|Casting|CastToBP_PlayerPerso Player))
  (Variables|/Game/FPMovement/Player/Blueprints/BP_PlayerPerso.BP_PlayerPerso_C|SetHasCrank _asbp_player_perso true)
  (Rendering|SetActorHiddenInGame true)
  (Collision|SetCollisionEnabled (Variables|Default|GetcollisionCrank) "NoCollision")
  (Actor|Tick|SetActorTickEnabled false))

(fn ConstructionScript)

(fn CanInteract?
  (return (not (Variables|Default|GetHasBeenPickedUp))))

(fn InteractPrompt
  (return true "Ramasser la manivelle"))