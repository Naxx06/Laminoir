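; BP_gramophone is an interactable gramophone that accepts the player's vinyl record to trigger the final sequence and unlock a door.
; On interact, it consumes the player's vinyl, shows the record mesh with a looping animation and prevents further interaction.
; It then switches the level's BP_MirrorDoorSequence to its FinalSequence state, plays the gramophone sound and unlocks the referenced door after a short delay.
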(event EventBeginPlay)

(event Collision|EventActorBeginOverlap
  (params (OtherActor :type Actor%20Object%20Reference)))

(event EventTick
  (params (DeltaSeconds :type Float%20%28single-precision%29)))

(event EventInteract
  (params (Player :type BP%20Player%20Perso%20Object%20Reference))
  (bind _vinylmesh (Variables|Default|GetVinylMesh))
  (if (not (Variables|Default|GetHasVinylInserted))
    (if (Variables|/Game/FPMovement/Player/Blueprints/BP_PlayerPerso.BP_PlayerPerso_C|GetHasVinyl Player)
      (Variables|/Game/FPMovement/Player/Blueprints/BP_PlayerPerso.BP_PlayerPerso_C|SetHasVinyl Player false)
      (Variables|Default|SetHasVinylInserted true)
      (Development|SetHiddeninGame _vinylmesh false false)
      (Rendering|SetVisibility _vinylmesh true false)
      (Components|Animation|PlayAnimation _vinylmesh "/Game/Fab/_Anisotropic__Record_test/anisotropic_record_test/SkeletalMeshes/anisotropic_record_test_Anim.anisotropic_record_test_Anim" true)
      (bind _returnvalue (Actor|GetActorOfClass "/Game/Art/BP/Animation_Door_Reflet/BP_MirrorDoorSequence.BP_MirrorDoorSequence_C"))
      (bind _output_get (Variables|Default|SetMirrorDoorSequenceRef _returnvalue))
      (Utilities|IsValid _output_get
        (:Is%20Valid
          ;[0 0 0 0.5] State FinalSequence
          (Variables|/Game/Art/BP/Animation_Door_Reflet/BP_MirrorDoorSequence.BP_MirrorDoorSequence_C|SetCurrentGameplayState (Variables|Default|GetMirrorDoorSequenceRef) "NewEnumerator5")
          (Default|ApplyGameplayState (Variables|Default|GetMirrorDoorSequenceRef))
          (Audio|PlaySound2D "/Game/Art/BP/Gramophone/Gramophone_Sound.Gramophone_Sound" 1.0 1.0 0.0 0 0)
          (Utilities|FlowControl|Delay 2.0)
          (Default|UnlockDoor (Variables|Default|GetDoorReference)))
        (:Is%20Not%20Valid
          (Development|PrintString "mirrorsequence not found" true true "(R=1.000000,G=0.000000,B=0.020864,A=1.000000)"))))))

(fn ConstructionScript)

(fn CanInteract?
  (return (not (Variables|Default|GetHasVinylInserted))))

(fn InteractPrompt
  (return true "Insérer le vinyle"))