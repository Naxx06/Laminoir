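; Configurable painting actor that displays a chosen texture on its canvas mesh.
; The construction script creates a dynamic instance of the MM_tableau material on the first slot of CanvaMesh.
; It feeds the painting texture, tiling, offset and rotation variables into that material's parameters.
; The event graph has no active logic, so all setup happens at construction.
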(event EventBeginPlay)

(event Collision|EventActorBeginOverlap
  (params (OtherActor :type Actor%20Object%20Reference)))

(event EventTick
  (params (DeltaSeconds :type Float%20%28single-precision%29)))

(fn ConstructionScript
  (bind _paintingtiling (Variables|Default|GetPaintingTiling))
  (bind _paintingoffset (Variables|Default|GetPaintingOffset))
  (bind (_x _y) (Math|Vector2D|BreakVector2D _paintingoffset))
  (bind (_x_2 _y_2) (Math|Vector2D|BreakVector2D _paintingtiling))
  (bind _returnvalue (Rendering|Material|CreateDynamicMaterialInstance (Variables|Default|GetCanvaMesh) 0 "/Game/Art/Materials/MM_tableau.MM_tableau" "None" :!class /Script/Engine.PrimitiveComponent))
  (Rendering|Material|SetTextureParameterValue _returnvalue "Texture_BaseColor" (Variables|Default|GetPaintingTexture))
  (Rendering|Material|SetScalarParameterValue _returnvalue "X Tile" _x_2 :!class /Script/Engine.MaterialInstanceDynamic)
  (Rendering|Material|SetScalarParameterValue _returnvalue "Y Tile" _y_2 :!class /Script/Engine.MaterialInstanceDynamic)
  (Rendering|Material|SetScalarParameterValue _returnvalue "X Offset" _x :!class /Script/Engine.MaterialInstanceDynamic)
  (Rendering|Material|SetScalarParameterValue _returnvalue "Y Offset" _y :!class /Script/Engine.MaterialInstanceDynamic)
  (Rendering|Material|SetScalarParameterValue _returnvalue "Rotation" (Variables|Default|GetPaintingRotation) :!class /Script/Engine.MaterialInstanceDynamic))