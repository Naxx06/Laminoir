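; BP_ElevatorTransitionManager runs the elevator cinematic that moves the player from the hotel hall to floor 11.
; StartElevatorCinematic locks input, preloads Level_etage11 hidden, fades out, reveals the cinematic-only actors and plays the level sequence.
; When the sequence finishes, it cuts to black, hides those actors, fades ambient audio, shows the new level and teleports the player to the arrival target.
; It then unloads the hall level, restores input and fades in.
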(event Custom|StartElevatorCinematic
  (bind _returnvalue (Game|GetPlayerController 0))
  (bind _elevatorsequenceref (Variables|Default|GetElevatorSequenceRef))
  (bind _sequenceplayer (Variables|/Script/LevelSequence.LevelSequenceActor|GetSequencePlayer _elevatorsequenceref))
  (Input|SetIgnoreMoveInput _returnvalue true)
  (Input|SetIgnoreLookInput _returnvalue true)
  (Game|LoadStreamLevel(byName) "Level_etage11" false)
  (CameraFades|StartCameraFade :self (Game|GetPlayerCameraManager 0) :ToAlpha 1.0 :Duration 2.0 :bHoldWhenFinished true)
  (Utilities|FlowControl|Delay 2.0)
  (Utilities|IsValid _elevatorsequenceref
    (:Is%20Valid
      (EventDispatchers|BindEventtoOnFinished _sequenceplayer (delegate Custom|FinishElevatorCinematic))
      (CallFunction|ShowcinematicActors true)
      (Sequencer|Player|Play _sequenceplayer :!class /Script/MovieScene.MovieSceneSequencePlayer)
      (CameraFades|StartCameraFade :self (Game|GetPlayerCameraManager 0) :FromAlpha 1.0 :Duration 5.0))))

(event Custom|FinishElevatorCinematic
  (bind _returnvalue (Game|GetPlayerCharacter 0))
  (bind _returnvalue_2 (Game|GetPlayerController 0))
  (bind _arrivaltargetref (Variables|Default|GetArrivalTargetRef))
  (bind _returnvalue_3 (Transformation|GetActorRotation _arrivaltargetref))
  (Utilities|FlowControl|Delay 0.05)
  (Class|PlayerCameraManager|SetManualCameraFade :self (Game|GetPlayerCameraManager 0) :InFadeAmount 1.0)
  (Utilities|FlowControl|Delay 0.1)
  (CallFunction|ShowcinematicActors false)
  (Audio|Components|Audio|FadeOut (Variables|/Script/Engine.AmbientSound|GetAudioComponent (Variables|Default|GetPersistentAmbiantSound)) 1.0 0.0 "Linear" :!class /Script/Engine.AudioComponent)
  (Variables|/Script/Engine.LevelStreaming|SetbShouldBeVisible (Class|GameplayStatics|GetStreamingLevel "Level_etage11") true)
  (Utilities|FlowControl|Delay 0.2)
  (Utilities|IsValid (Variables|Default|GetArrivalTargetRef)
    (:Is%20Valid
      (Components|Movement|StopMovementImmediately (Variables|/Script/Engine.Character|GetCharacterMovement _returnvalue))
      (Transformation|SetActorLocationAndRotation _returnvalue (Transformation|GetActorLocation _arrivaltargetref) _returnvalue_3 false true)
      (Pawn|SetControlRotation _returnvalue_2 _returnvalue_3)
      (Game|UnloadStreamLevel(byName) "Slvl_Hall_Hotel" false)
      (Development|PrintString "Hall_decharge")
      (Game|Player|SetViewTargetwithBlend _returnvalue_2 _returnvalue 0.0 "VTBlend_Linear" 0.0 false)
      (Utilities|FlowControl|Delay 0.5)
      (Input|ResetIgnoreMoveInput _returnvalue_2)
      (Input|ResetIgnoreLookInput _returnvalue_2)
      (CameraFades|StartCameraFade :self (Game|GetPlayerCameraManager 0) :FromAlpha 1.0 :Duration 2.0))))

(event Custom|ShowcinematicActors
  (params (Visible :type Boolean))
  (for _array_element (Variables|Default|GetCinematicActors)
    (Rendering|SetActorHiddenInGame _array_element (not Visible))))

(event EventBeginPlay
  (CallFunction|ShowcinematicActors false))

(fn ConstructionScript)