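; Interactable elevator that closes its doors and starts a transition cinematic when used with the player inside.
; An overlap volume tracks whether BP_PlayerPerso is inside, and interacting then triggers the sequence only once.
; A timeline lerps both doors from their initial open rotations to closed ones alongside a sound.
; When the timeline finishes, it calls StartElevatorCinematic on the BP_ElevatorTransitionManager found at BeginPlay.
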(event OnComponentBeginOverlap(PlayerCollision)
  (params (OverlappedComponent :type Primitive%20Component%20Object%20Reference) (OtherActor :type Actor%20Object%20Reference) (OtherComp :type Primitive%20Component%20Object%20Reference) (OtherBodyIndex :type Integer) (bFromSweep :type Boolean) (SweepResult :type Hit%20Result%20Structure%20%28by%20ref%29))
  (Utilities|Casting|CastToBP_PlayerPerso OtherActor)
  (Variables|Default|SetPlayerInside true))

(event OnComponentEndOverlap(PlayerCollision)
  (params (OverlappedComponent :type Primitive%20Component%20Object%20Reference) (OtherActor :type Actor%20Object%20Reference) (OtherComp :type Primitive%20Component%20Object%20Reference) (OtherBodyIndex :type Integer))
  (Utilities|Casting|CastToBP_PlayerPerso OtherActor)
  (Variables|Default|SetPlayerInside false))

(event Custom|CloseDoors
  (bind _transitionmanagerref (Variables|Default|GetTransitionManagerRef))
  (Audio|PlaySound2D "/Game/Art/Sounds/Elevator_Door_ODC-0019-355.Elevator_Door_ODC-0019-355" 1.0 1.0 0.0 0 0)
  (bind _alpha (Timeline|TL_ElevatorDoors Play)
    (:Update
      (Utilities|FlowControl|Sequence
        (:then_0
          (Transformation|SetRelativeRotation (Variables|Default|GetDoorLeft) (Math|Rotator|Lerp(Rotator) (Variables|Default|GetDoorLeftOpenRotation) (Variables|Default|GetDoorLeftClosedRotation) _alpha true) false false))
        (:then_1
          (Transformation|SetRelativeRotation (Variables|Default|GetDoorRight) (Math|Rotator|Lerp(Rotator) (Variables|Default|GetDoorRightOpenRotation) (Variables|Default|GetDoorRightClosedRotation) _alpha true) false false))))
    (:Finished
      (Utilities|IsValid _transitionmanagerref
        (:Is%20Valid
          (Default|StartElevatorCinematic _transitionmanagerref))))))

(event EventBeginPlay
  (Utilities|FlowControl|Sequence
    (:then_0
      (Variables|Default|SetDoorLeftOpenRotation (Variables|/Script/Engine.SceneComponent|GetRelativeRotation (Variables|Default|GetDoorLeft))))
    (:then_1
      (Variables|Default|SetDoorRightOpenRotation (Variables|/Script/Engine.SceneComponent|GetRelativeRotation (Variables|Default|GetDoorRight))))
    (:then_2
      (bind _returnvalue (Actor|GetActorOfClass "/Game/Art/BP/Ascenseur/BP_ElevatorTransitionManager.BP_ElevatorTransitionManager_C"))
      (Variables|Default|SetTransitionManagerRef _returnvalue))))

(event EventInteract
  (params (Player :type BP%20Player%20Perso%20Object%20Reference))
  (if (and (Variables|Default|GetPlayerInside) (not (Variables|Default|GetSequenceStarted)))
    (Variables|Default|SetSequenceStarted true)
    (CallFunction|CloseDoors)))

(fn ConstructionScript)

(fn CanInteract?
  (return true))

(fn InteractPrompt
  (return true "Appuyer"))