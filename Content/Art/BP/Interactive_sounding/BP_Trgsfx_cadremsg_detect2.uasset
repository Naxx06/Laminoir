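; Trigger actor that plays a one-time "cadre msg detect2" sound when its box is overlapped during a specific state of the mirror door sequence.
; On BeginPlay it caches the BP_MirrorDoorSequence actor.
; Box overlap checks that actor's CurrentGameplayState, then a DoOnce plays Audio, followed by AudioEcho one second later.
; The overlap does not filter the overlapping actor, and debug strings report each outcome.
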(event OnComponentBeginOverlap(Box)
  (params (OverlappedComponent :type Primitive%20Component%20Object%20Reference) (OtherActor :type Actor%20Object%20Reference) (OtherComp :type Primitive%20Component%20Object%20Reference) (OtherBodyIndex :type Integer) (bFromSweep :type Boolean) (SweepResult :type Hit%20Result%20Structure%20%28by%20ref%29))
  (Development|PrintString "trgsfx_cadre_detect" true true "(R=1.000000,G=0.000000,B=0.020864,A=1.000000)")
  (if (Utilities|Enum|Equal(Enum) (Variables|/Game/Art/BP/Animation_Door_Reflet/BP_MirrorDoorSequence.BP_MirrorDoorSequence_C|GetCurrentGameplayState (Variables|Default|GetMirrorDoorSequenceRef)) "NewEnumerator1")
    (Utilities|FlowControl|DoOnce false
      (:Completed
        (Audio|Components|Audio|Play (Variables|Default|GetAudio) 0.0)
        (Utilities|FlowControl|Delay 1.0)
        (Audio|Components|Audio|Play (Variables|Default|GetAudioEcho) 0.0)
        (Development|PrintString "msg detect2 played" true true "(R=0.298868,G=1.000000,B=0.185537,A=1.000000)")))
    (else
      (Development|PrintString "Wrong state" true true "(R=1.000000,G=0.081581,B=0.000000,A=1.000000)"))))

(event EventBeginPlay
  ;[0.15 0.15 0.15 0.5] Comment
  (bind _returnvalue (Actor|GetActorOfClass "/Game/Art/BP/Animation_Door_Reflet/BP_MirrorDoorSequence.BP_MirrorDoorSequence_C"))
  (Variables|Default|SetMirrorDoorSequenceRef _returnvalue))

(event EventTick
  (params (DeltaSeconds :type Float%20%28single-precision%29)))

(fn ConstructionScript)