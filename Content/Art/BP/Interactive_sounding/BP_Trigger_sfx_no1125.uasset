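; Trigger actor that plays sound effect no1125 once when something overlaps its box during a specific phase of the mirror door sequence.
; BeginPlay caches the level's BP_MirrorDoorSequence actor.
; On overlap, it checks that sequence's current gameplay state and plays the Audio component through a DoOnce only in the matching state, printing debug messages for success, wrong state or missing reference.
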(event OnComponentBeginOverlap(Box)
  (params (OverlappedComponent :type Primitive%20Component%20Object%20Reference) (OtherActor :type Actor%20Object%20Reference) (OtherComp :type Primitive%20Component%20Object%20Reference) (OtherBodyIndex :type Integer) (bFromSweep :type Boolean) (SweepResult :type Hit%20Result%20Structure%20%28by%20ref%29))
  (Development|PrintString "No1125" true true "(R=1.000000,G=0.000000,B=0.020864,A=1.000000)")
  (Utilities|IsValid (Variables|Default|GetMirrorDoorSequenceRef)
    (:Is%20Valid
      (if (Utilities|Enum|Equal(Enum) (Variables|/Game/Art/BP/Animation_Door_Reflet/BP_MirrorDoorSequence.BP_MirrorDoorSequence_C|GetCurrentGameplayState (Variables|Default|GetMirrorDoorSequenceRef)) "NewEnumerator1")
        (Utilities|FlowControl|DoOnce false
          (:Completed
            (Audio|Components|Audio|Play (Variables|Default|GetAudio) 0.0)
            (Development|PrintString "sfx no1125 played")))
        (else
          (Development|PrintString "sfx no1125 wrong state" true true "(R=1.000000,G=0.043073,B=0.000000,A=1.000000)"))))
    (:Is%20Not%20Valid
      (Development|PrintString "MirrorDoorSequence not valid"))))

(event EventBeginPlay
  (bind _returnvalue (Actor|GetActorOfClass "/Game/Art/BP/Animation_Door_Reflet/BP_MirrorDoorSequence.BP_MirrorDoorSequence_C"))
  (bind _output_get (Variables|Default|SetMirrorDoorSequenceRef _returnvalue))
  (Utilities|IsValid _output_get))

(event EventTick
  (params (DeltaSeconds :type Float%20%28single-precision%29)))

(fn ConstructionScript)