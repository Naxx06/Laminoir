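; Trigger actor that plays a sound effect for the empty corridor when its box volume is overlapped during a specific stage of the mirror door sequence.
; On BeginPlay it finds and caches the level's BP_MirrorDoorSequence and prints whether the reference is valid.
; On overlap it checks that actor's CurrentGameplayState against one enum value, then plays its Audio component through a DoOnce so it fires only once.
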(event OnComponentBeginOverlap(Box)
  (params (OverlappedComponent :type Primitive%20Component%20Object%20Reference) (OtherActor :type Actor%20Object%20Reference) (OtherComp :type Primitive%20Component%20Object%20Reference) (OtherBodyIndex :type Integer) (bFromSweep :type Boolean) (SweepResult :type Hit%20Result%20Structure%20%28by%20ref%29))
  (Development|PrintString "EmptyCorridor" true true "(R=1.000000,G=0.000000,B=0.020864,A=1.000000)")
  (if (Utilities|Enum|Equal(Enum) (Variables|/Game/Art/BP/Animation_Door_Reflet/BP_MirrorDoorSequence.BP_MirrorDoorSequence_C|GetCurrentGameplayState (Variables|Default|GetMirrorDoorSequenceRef)) "NewEnumerator1")
    (Utilities|FlowControl|DoOnce false
      (:Completed
        (Audio|Components|Audio|Play (Variables|Default|GetAudio) 0.0)))))

(event EventBeginPlay
  (bind _returnvalue (Actor|GetActorOfClass "/Game/Art/BP/Animation_Door_Reflet/BP_MirrorDoorSequence.BP_MirrorDoorSequence_C"))
  (bind _output_get (Variables|Default|SetMirrorDoorSequenceRef _returnvalue))
  (Utilities|IsValid _output_get
    (:Is%20Valid
      (Development|PrintString "hint good valid"))
    (:Is%20Not%20Valid
      (Development|PrintString "hint good not valid" true true "(R=1.000000,G=0.162433,B=0.120399,A=1.000000)"))))

(event EventTick
  (params (DeltaSeconds :type Float%20%28single-precision%29)))

(fn ConstructionScript)