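; Planar mirror actor that shows a live reflection using a scene capture rendered into a dynamic material on the mirror plane.
; Each tick, it reflects the first-person camera's transform through actor local space to place the capture.
; An optional clip plane cuts geometry behind the mirror; a helper for hiding static meshes there is never called here.
; Looping timers resize the render target as quality or, optionally, viewport size changes.
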(event EventBeginPlay
  (Utilities|FlowControl|Sequence
    (:then_0
      (CallFunction|CreateMaterialandRenderTarget)
      (CallFunction|SetComponentVisibilities)
      (CallFunction|GetPlayerReferences)
      (CallFunction|SetClipPlane))
    (:then_1
      (if (Variables|Default|GetUseViewportSize)
        (Utilities|Time|SetTimerbyFunctionName 0 "UpdateViewportSizeOnChange" 0.2 true))
      (Utilities|Time|SetTimerbyFunctionName 0 "UpdateResolutionQuality" 0.2 true)
      (Actor|Tick|SetActorTickEnabled true))))

(event EventTick
  (params (DeltaSeconds :type Float%20%28single-precision%29))
  (CallFunction|UpdateSceneCaptureLocationRotation))

(fn ConstructionScript
  (Rendering|Material|SetScalarParameterValueonMaterials (Variables|Default|GetMirrorPlane) "RoundedCorners" (Variables|Default|GetRoundedCornersValue)))

(fn CalculateSceneCaptureLocation
  (params (Location%20In :type Vector))
  (bind _returnvalue (Transformation|GetActorTransform))
  (return (Math|Transform|TransformLocation _returnvalue (* (Math|Transform|InverseTransformLocation _returnvalue Location%20In) (Variables|Default|GetCameraInverseModifier)))))

(fn CalculateSceneCaptureRotation
  (params (Rotation%20In :type Rotator))
  (bind _returnvalue (Transformation|GetActorTransform))
  (bind (_x _y _z) (Math|Rotator|BreakRotIntoAxes Rotation%20In))
  (bind _camerainversemodifier (Variables|Default|GetCameraInverseModifier))
  (return (Math|Rotator|MakeRotfromXZ (Math|Transform|TransformDirection _returnvalue (* (Math|Transform|InverseTransformDirection _returnvalue _x) _camerainversemodifier)) (Math|Transform|TransformDirection _returnvalue (* (Math|Transform|InverseTransformDirection _returnvalue _z) _camerainversemodifier)))))

(fn SetPlayerCameraReference
  (params (Player%20Camera :type Camera%20Component%20Object%20Reference))
  ;[0.15 0.15 0.15 0.5] Go look at BP_FirstPersonCharacter for more about this. Essentially, it just receives a reference to the player's currently enabled camera.
  (Variables|Default|SetPlayerCameraRef Player%20Camera))

(fn GetPlayerReferences
  (bind _returnvalue (Actor|GetActorOfClass (Variables|/Script/Engine.GameModeBase|GetDefaultPawnClass (Game|GetGameMode))))
  (Utilities|IsValid _returnvalue
    (:Is%20Valid
      (bind _output_get (Variables|Default|SetPlayerActor _returnvalue))
      (bind _asbp_first_person_character (Utilities|Casting|CastToBP_FirstPersonCharacter _output_get))
      (Variables|Default|SetPlayerCameraRef (Variables|/Game/FirstPerson/Blueprints/BP_FirstPersonCharacter.BP_FirstPersonCharacter_C|GetFirstPersonCamera _asbp_first_person_character)))))

(fn SetComponentVisibilities
  ;[0.15 0.15 0.15 0.5] Important if you have several of the mirrors in the editor, or else it will end up lagging. This Blueprint's "MirrorCamera" (Scene Capture Component 2D) has "Visible" disabled for this reason. It will be enabled again here during BeginPlay.
  (Rendering|SetVisibility (Variables|Default|GetMirrorCamera) true false))

(fn SetClipPlane
  (bind _mirrorplane (Variables|Default|GetMirrorPlane))
  (bind _mirrorcamera (Variables|Default|GetMirrorCamera))
  ;[0.15 0.15 0.15 0.5] This is done so that the Scene Capture Component 2D that is behind the MirrorPlane doesn't render/show whatever is behind the MirrorPlane. The setting "Support global clip plane for Planar Reflections" in Project Settings has to be enabled as well for this to work.
  (Variables|/Script/Engine.SceneCaptureComponent2D|SetbEnableClipPlane _mirrorcamera (Variables|Default|GetEnableClipPlane))
  (Variables|/Script/Engine.SceneCaptureComponent2D|SetClipPlaneBase _mirrorcamera (Transformation|GetWorldLocation _mirrorplane))
  (Variables|/Script/Engine.SceneCaptureComponent2D|SetClipPlaneNormal _mirrorcamera (Math|Vector|GetUpVector _mirrorplane)))

(fn UpdateSceneCaptureLocationRotation
  (bind _playercameraref (Variables|Default|GetPlayerCameraRef))
  (Utilities|IsValid _playercameraref
    (:Is%20Valid
      (Transformation|SetWorldLocationAndRotation (Variables|Default|GetMirrorCamera) (CallFunction|CalculateSceneCaptureLocation (Transformation|GetWorldLocation _playercameraref)) (CallFunction|CalculateSceneCaptureRotation (Transformation|GetWorldRotation _playercameraref)) false false))))

(fn CreateMaterialandRenderTarget
  (bind _returnvalue (Viewport|GetViewportSize))
  (bind _rendertargetresolution (Variables|Default|GetRenderTargetResolution))
  (bind _quality (Variables|Default|GetQuality))
  (bind _returnvalue_2 (* _quality _rendertargetresolution))
  (bind _returnvalue_3 (Math|Float|Truncate _returnvalue_2))
  (if (Variables|Default|GetUseViewportSize)
    (bind _output_get (Variables|Default|SetCurrentViewportSize (Utilities|Struct|MakeIntVector2 (Math|Float|Truncate (.x _returnvalue)) (Math|Float|Truncate (.y _returnvalue)))))
    (Variables|Default|SetTargetRenderResolution (Utilities|Struct|MakeIntVector2 (Math|Float|Truncate (* (.x _output_get) _quality)) (Math|Float|Truncate (* (.y _output_get) _quality))))
    (else
      (Variables|Default|SetTargetRenderResolution (Utilities|Struct|MakeIntVector2 _returnvalue_3 _returnvalue_3))))
  (bind _returnvalue_4 (Rendering|CreateRenderTarget2D (.x (Variables|Default|GetTargetRenderResolution)) (.y (Variables|Default|GetTargetRenderResolution)) "RTF_RGBA16f" "(R=0.000000,G=0.000000,B=0.000000,A=1.000000)" false true))
  (bind _output_get_2 (Variables|/Script/Engine.SceneCaptureComponent2D|SetTextureTarget (Variables|Default|GetMirrorCamera) _returnvalue_4))
  (bind _output_get_3 (Variables|Default|SetRenderTargetTexture _output_get_2))
  (bind _returnvalue_5 (Rendering|Material|CreateDynamicMaterialInstance (Variables|Default|GetMirrorPlane) 0 "/Game/Mirror/M_Mirror.M_Mirror" "None" :!class /Script/Engine.PrimitiveComponent))
  (bind _output_get_4 (Variables|Default|SetMirrorMaterial _returnvalue_5))
  (Rendering|Material|SetTextureParameterValue _output_get_4 "RenderTarget" _output_get_3)
  (if (Variables|Default|GetUseViewportSize)
    (Rendering|Material|SetScalarParameterValue _output_get_4 "UseViewportSize" 1.0 :!class /Script/Engine.MaterialInstanceDynamic))
  (Rendering|Material|SetScalarParameterValue _output_get_4 "RoundedCorners" (Variables|Default|GetRoundedCornersValue) :!class /Script/Engine.MaterialInstanceDynamic))

(fn UpdateViewportSizeonChange
  (bind _returnvalue (Viewport|GetViewportSize))
  (bind _quality (Variables|Default|GetQuality))
  (bind _returnvalue_2 (Math|Float|Truncate (.x _returnvalue)))
  (bind _returnvalue_3 (Math|Float|Truncate (.y _returnvalue)))
  (if (Variables|Default|GetUseViewportSize)
    (if (or (!= _returnvalue_2 (.x (Variables|Default|GetCurrentViewportSize))) (!= _returnvalue_3 (.y (Variables|Default|GetCurrentViewportSize))))
      (Variables|Default|SetCurrentViewportSize (Utilities|Struct|MakeIntVector2 _returnvalue_2 _returnvalue_3))
      (bind _output_get (Variables|Default|SetTargetRenderResolution (Utilities|Struct|MakeIntVector2 (Math|Float|Truncate (* (.x _returnvalue) _quality)) (Math|Float|Truncate (* (.y _returnvalue) _quality)))))
      (Rendering|ResizeRenderTarget2D (Variables|/Script/Engine.SceneCaptureComponent2D|GetTextureTarget (Variables|Default|GetMirrorCamera)) (.x _output_get) (.y _output_get)))))

(fn UpdateResolutionQuality
  (bind _quality (Variables|Default|GetQuality))
  (bind _useviewportsize (Variables|Default|GetUseViewportSize))
  (bind _rendertargetresolution (Variables|Default|GetRenderTargetResolution))
  (bind _currentviewportsize (Variables|Default|GetCurrentViewportSize))
  (bind _returnvalue (select _useviewportsize (Utilities|Struct|MakeIntVector2 (.x _currentviewportsize) (.y _currentviewportsize)) (Utilities|Struct|MakeIntVector2 _rendertargetresolution _rendertargetresolution)))
  (bind _returnvalue_2 (* (.x _returnvalue) _quality))
  (bind _returnvalue_3 (* (.y _returnvalue) _quality))
  (bind _returnvalue_4 (Math|Float|Truncate _returnvalue_2))
  (bind _returnvalue_5 (Math|Float|Truncate _returnvalue_3))
  (if (Variables|Default|GetUpdateQuality)
    (if (or (!= (.x (Variables|Default|GetTargetRenderResolution)) _returnvalue_4) (!= (.y (Variables|Default|GetTargetRenderResolution)) _returnvalue_5))
      (bind _output_get (Variables|Default|SetTargetRenderResolution (Utilities|Struct|MakeIntVector2 _returnvalue_4 _returnvalue_5)))
      (Rendering|ResizeRenderTarget2D (Variables|/Script/Engine.SceneCaptureComponent2D|GetTextureTarget (Variables|Default|GetMirrorCamera)) (.x _output_get) (.y _output_get)))))

(fn HideAllStaticMeshActorsBehindMirror
  (bind _index (LocalVariables|GetIndex))
  (bind _outactors (Actor|GetAllActorsOfClass "/Script/Engine.StaticMeshActor"))
  (for _array_element _outactors
    (if (and (Utilities|IsValid _array_element) (< (Math|Vector|DotProduct (Math|Vector|Normalize (- (Transformation|GetWorldLocation (Variables|/Script/Engine.StaticMeshActor|GetStaticMeshComponent _array_element)) (Transformation|GetActorLocation))) (Math|Vector|GetForwardVector (Variables|Default|GetDefaultSceneRoot))) 0.0))
      (Utilities|Array|SetArrayElem (Variables|Default|GetActorsToHide) _index _array_element true)
      (Math|Integer|IncrementInt _index)))
  (Variables|/Script/Engine.SceneCaptureComponent|SetHiddenActors (Variables|Default|GetMirrorCamera) (Variables|Default|GetActorsToHide)))